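; Gameplay ability for enemy melee attacks, which turns the avatar toward its combat target and plays a random tagged attack montage.
; A gameplay event matching the montage tag triggers a small sphere query at that tag's combat socket.
; Live players found there, excluding the avatar, take damage through CauseDamage.
; The ability ends after that hit event or when the montage completes, is interrupted or is cancelled.
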(event Ability|EventActivateAbility
  (bind _returnvalue (Ability|GetAvatarActorfromActorInfo))
  (bind _returnvalue_2 (Class|EnemyInterface|GetCombatTarget(Message) (Ability|GetAvatarActorfromActorInfo)))
  (bind _output_get (Variables|Default|SetCombatTarget _returnvalue_2))
  (Utilities|IsValid _output_get
    (:Is%20Valid
      (bind _ascombat_interface (Utilities|Casting|CastToCombatInterface (Ability|GetAvatarActorfromActorInfo)))
      (Class|CombatInterface|UpdateFacingTarget _ascombat_interface (Transformation|GetActorLocation (Variables|Default|GetCombatTarget)))
      (bind _returnvalue_3 (Class|CombatInterface|GetAttackMontages _ascombat_interface))
      (Variables|Default|SetMontage%20Tag (.MontageTag (Utilities|Struct|BreakTaggedMontage (Class|AuraDamageGameplayAbility|GetRandomTaggedMontagefromArray _returnvalue_3))))
      (|PlayMontageandWaitProxy "None" (.Montage (Utilities|Struct|BreakTaggedMontage (Class|AuraDamageGameplayAbility|GetRandomTaggedMontagefromArray _returnvalue_3))) 1.0 "None" false 1.0 0.0 false
        (:then
          (Ability|Tasks|WaitGameplayEvent (Variables|Default|GetMontage%20Tag) 0
            (:EventReceived
              (Utilities|FlowControl|Sequence
                (:then_0
                  (bind _returnvalue_4 (Class|CombatInterface|GetCombatSocketLocation(Message) _returnvalue (Variables|Default|GetMontage%20Tag)))
                  (bind _outoverlappingactors (Class|AuraAbilitySystemLibrary|GetLivePlayersWithinRadius self (Utilities|Array|MakeArray _returnvalue) 45.0 _returnvalue_4))
                  (for _array_element _outoverlappingactors
                    (Class|AuraDamageGameplayAbility|CauseDamage _array_element)))
                (:then_1
                  (Ability|EndAbility))))))
        (:OnCompleted
          (Ability|EndAbility :!label _label))
        (:OnInterrupted
          (goto _label))
        (:OnCancelled
          (goto _label))))))

(event Ability|EventOnEndAbility
  (params (bWasCancelled :type Boolean)))

(fn FGetRandomMontagetoPlay
  (params (Montages :type Array%20of%20Tagged%20Montage%20Structures))
  (bind _returnvalue (Utilities|Array|Length Montages))
  (bind _returnvalue_2 (- _returnvalue 1))
  (bind _returnvalue_3 (Math|Random|RandomIntegerinRange 0 _returnvalue_2))
  (bind _output (Utilities|Array|Get(acopy) Montages _returnvalue_3))
  (bind (_montage _montagetag) (Utilities|Struct|BreakTaggedMontage _output))
  (Utilities|FlowControl|Sequence
    (:then_0
      (LocalVariables|SetRetMonatge _montage)
      (LocalVariables|SetRetMontageTag _montagetag))
    (:then_1
      (return (LocalVariables|GetRetMontageTag) (LocalVariables|GetRetMonatge)))))