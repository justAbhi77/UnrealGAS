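; Enemy gameplay ability for a ranged attack that fires a projectile at the avatar's combat target.
; If the target is valid, it turns the avatar toward it through CombatInterface and plays a random tagged attack montage.
; A gameplay event matching the montage tag triggers SpawnProjectile from the tagged socket, with optional pitch override, then ends the ability.
; Montage interruption or cancellation also ends the ability.
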(event Ability|EventActivateAbility
  (bind _returnvalue (Class|EnemyInterface|GetCombatTarget(Message) (Ability|GetAvatarActorfromActorInfo)))
  (bind _output_get (Variables|Default|SetCombatTarget _returnvalue))
  (Utilities|IsValid _output_get
    (:Is%20Valid
      (bind _ascombat_interface (Utilities|Casting|CastToCombatInterface (Ability|GetAvatarActorfromActorInfo)))
      (Class|CombatInterface|UpdateFacingTarget _ascombat_interface (Transformation|GetActorLocation (Variables|Default|GetCombatTarget)))
      (bind _returnvalue_2 (Class|CombatInterface|GetAttackMontages _ascombat_interface))
      (Variables|Default|SetMontage%20Tag (.MontageTag (Utilities|Struct|BreakTaggedMontage (Class|AuraDamageGameplayAbility|GetRandomTaggedMontagefromArray _returnvalue_2))))
      (Variables|Default|SetSocket%20Tag (.SocketTag (Utilities|Struct|BreakTaggedMontage (Class|AuraDamageGameplayAbility|GetRandomTaggedMontagefromArray _returnvalue_2))))
      (|PlayMontageandWaitProxy "None" (.Montage (Utilities|Struct|BreakTaggedMontage (Class|AuraDamageGameplayAbility|GetRandomTaggedMontagefromArray _returnvalue_2))) 1.0 "None" false 1.0 0.0 false
        (:then
          (Ability|Tasks|WaitGameplayEvent (Variables|Default|GetMontage%20Tag) 0 true
            (:EventReceived
              (Utilities|FlowControl|Sequence
                (:then_0
                  (Class|AuraProjectileSpell|SpawnProjectile (Transformation|GetActorLocation (Variables|Default|GetCombatTarget)) (Variables|Default|GetSocket%20Tag) (Variables|Default|GetbShouldOverridePitch) (Variables|Default|GetPitchOverride)))
                (:then_1
                  (Ability|EndAbility))))))
        (:OnInterrupted
          (Ability|EndAbility :!label _label))
        (:OnCancelled
          (goto _label))))))

(event Ability|EventOnEndAbility
  (params (bWasCancelled :type Boolean)))