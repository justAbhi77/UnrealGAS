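; Enemy gameplay ability for a shaman that summons random minions around itself when it has a valid combat target.
; It shuffles the spawn locations, plays a ground-summon Niagara effect at each, then starts the summon montage.
; On the montage's attack gameplay event, a self-calling delayed custom-event loop staggers minion spawns, each facing the target with a default controller.
; EndAbility is only called when the target is invalid.
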(event Custom|eLoop
  (bind _spawnlocations (Variables|Default|GetSpawnLocations))
  (bind _spawnlocatioindex (Variables|Default|GetSpawnLocatioIndex))
  (bind _output (Utilities|Array|Get(acopy) _spawnlocations _spawnlocatioindex))
  (bind _location (Math|Transform|BreakTransform _output))
  (bind _returnvalue (+ _location "0.000000,0.000000,100.000000"))
  (if (< (Variables|Default|GetSpawnLocatioIndex) (Utilities|Array|Length (Variables|Default|GetSpawnLocations)))
    (Utilities|FlowControl|Sequence
      (:then_0
        (bind _returnvalue_2 (Game|SpawnActorfromClass (Class|AuraSummonAbility|GetRandomMinionClass) (Math|Transform|MakeTransform _returnvalue (Math|Rotator|FindLookatRotation _returnvalue (Transformation|GetActorLocation (Variables|Default|GetCombatTarget))) "1.000000,1.000000,1.000000") "AlwaysSpawn" "MultiplyWithRoot" 0 0))
        (Utilities|IsValid _returnvalue_2
          (:Is%20Valid
            (Pawn|SpawnDefaultController _returnvalue_2))))
      (:then_1
        (Math|Integer|IncrementInt (Variables|Default|GetSpawnLocatioIndex)
          (:%20%20
            (Utilities|FlowControl|Delay 0.2)
            (CallFunction|ELoop)))))))

(event Ability|EventActivateAbility
  (bind _returnvalue (Class|EnemyInterface|GetCombatTarget(Message) (Ability|GetAvatarActorfromActorInfo)))
  (bind _output_get (Variables|Default|SetCombatTarget _returnvalue))
  (Utilities|IsValid _output_get
    (:Is%20Valid
      (bind _returnvalue_2 (Class|AuraSummonAbility|GetSpawnLocations))
      (bind _output_get_2 (Variables|Default|SetSpawnLocations _returnvalue_2))
      (Utilities|Array|Shuffle _output_get_2)
      (Utilities|FlowControl|Sequence
        (:then_0
          (for _array_element (Variables|Default|GetSpawnLocations)
            (Niagara|SpawnSystematLocation "/Game/Assets/Effects/Combat/NS_GroundSummon.NS_GroundSummon" (.Location (Math|Transform|BreakTransform _array_element)) (.Rotation (Math|Transform|BreakTransform _array_element)))))
        (:then_1
          (|PlayMontageandWaitProxy "None" "/Game/Assets/Enemies/Shaman/Animations/AM_Shaman_Summon.AM_Shaman_Summon" 1.0 "None" true 1.0 0.0 false
            (:then
              (Ability|Tasks|WaitGameplayEvent "(TagName=\"Montage.Attack.1\")" 0
                (:EventReceived
                  (if (< (Variables|Default|GetSpawnLocatioIndex) (Utilities|Array|Length (Variables|Default|GetSpawnLocations)))
                    (Utilities|FlowControl|Sequence
                      (:then_0
                        (bind _returnvalue_3 (Game|SpawnActorfromClass (Class|AuraSummonAbility|GetRandomMinionClass) (Math|Transform|MakeTransform (+ (.Location (Math|Transform|BreakTransform (Utilities|Array|Get(acopy) (Variables|Default|GetSpawnLocations) (Variables|Default|GetSpawnLocatioIndex)))) "0.000000,0.000000,100.000000") (Math|Rotator|FindLookatRotation (+ (.Location (Math|Transform|BreakTransform (Utilities|Array|Get(acopy) (Variables|Default|GetSpawnLocations) (Variables|Default|GetSpawnLocatioIndex)))) "0.000000,0.000000,100.000000") (Transformation|GetActorLocation (Variables|Default|GetCombatTarget))) "1.000000,1.000000,1.000000") "AlwaysSpawn" "MultiplyWithRoot" 0 0))
                        (Utilities|IsValid _returnvalue_3
                          (:Is%20Valid
                            (Pawn|SpawnDefaultController _returnvalue_3))))
                      (:then_1
                        (Math|Integer|IncrementInt (Variables|Default|GetSpawnLocatioIndex)
                          (:%20%20
                            (Utilities|FlowControl|Delay 0.2)
                            (CallFunction|ELoop)))))))))))))
    (:Is%20Not%20Valid
      (Ability|EndAbility))))

(event Ability|EventOnEndAbility
  (params (bWasCancelled :type Boolean)))