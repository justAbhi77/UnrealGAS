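; GA_HitReact is a gameplay ability that plays a hit reaction on its avatar actor.
; On activation it applies GE_HitReact to the owner, keeps the handle, and plays the montage the avatar supplies through GetHitReactMontage.
; When the montage completes, is interrupted or is cancelled, it removes that effect and ends the ability.
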(event Ability|EventActivateAbility
  (|CallParentFunction)
  (bind _returnvalue (Ability|ApplyGameplayEffectToOwner "/Game/Blueprints/AbilitySystem/GameplayEffects/GE_HitReact.GE_HitReact_C"))
  (Variables|Default|SetActiveGeHitReact _returnvalue)
  (bind _returnvalue_2 (Class|CombatInterface|GetHitReactMontage(Message) (Ability|GetAvatarActorfromActorInfo)))
  (|PlayMontageandWaitProxy "None" _returnvalue_2 1.0 "None" true 1.0 0.0 false
    (:OnCompleted
      _)
    (:OnInterrupted
      _)
    (:OnCancelled
      _))
  (Ability|RemoveGameplayEffectFromOwnerWithHandle (Variables|Default|GetActiveGeHitReact))
  (Ability|EndAbility))

(event Ability|EventOnEndAbility
  (params (bWasCancelled :type Boolean))
  (|CallParentFunction bWasCancelled))