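; Melee attack gameplay ability that faces the avatar toward its combat target and plays the goblin spear attack montage.
; Target, facing and socket location come through combat interface calls on the avatar.
; On the melee montage gameplay event it only draws a debug sphere at the combat socket, with no damage, then ends.
; EndAbility is reached only through that event, so an invalid target leaves the ability active.
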(event Ability|EventActivateAbility
  (bind _returnvalue (Class|EnemyInterface|GetCombatTarget(Message) (Ability|GetAvatarActorfromActorInfo)))
  (bind _output_get (Variables|Default|SetCombatTarget _returnvalue))
  (Utilities|IsValid _output_get
    (:Is%20Valid
      (bind _ascombat_interface (Utilities|Casting|CastToCombatInterface (Ability|GetAvatarActorfromActorInfo)))
      (Class|CombatInterface|UpdateFacingTarget _ascombat_interface (Transformation|GetActorLocation (Variables|Default|GetCombatTarget)))
      (|PlayMontageandWaitProxy "None" "/Game/Assets/Enemies/Goblin/Animations/Spear/AM_Attack_GoblinSpear.AM_Attack_GoblinSpear" 1.0 "None" true 1.0 0.0 false
        (:then
          (Ability|Tasks|WaitGameplayEvent "(TagName=\"Event.Montage.Attack.Melee\")" 0
            (:EventReceived
              (Utilities|FlowControl|Sequence
                (:then_0
                  (bind _returnvalue_2 (Class|CombatInterface|GetCombatSocketLocation(Message) (Ability|GetAvatarActorfromActorInfo)))
                  (Rendering|Debug|DrawDebugSphere _returnvalue_2 15.0 12 "(R=1.000000,G=0.000000,B=0.045847,A=1.000000)" 3.0))
                (:then_1
                  (Ability|EndAbility))))))))))

(event Ability|EventOnEndAbility
  (params (bWasCancelled :type Boolean)))