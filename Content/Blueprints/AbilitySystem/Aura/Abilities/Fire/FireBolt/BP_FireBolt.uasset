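; BP_FireBolt is the Blueprint actor for the FireBolt fire ability, with a check that destroys it once it stops moving.
; Every Tick, FCheckNoMove compares the actor's current location with the previous frame's.
; When the distance is at or below MinDistancePerFrame, it spawns the impact sound and effect at that location and destroys the actor.
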(event EventTick
  (params (DeltaSeconds :type Float%20%28single-precision%29))
  (CallFunction|FCheckNoMove))

(fn ConstructionScript)

(fn FCheckNoMove
  (Variables|Default|SetLocationLastFrame (Variables|Default|GetLocationThisFrame))
  (Variables|Default|SetLocationThisFrame (Transformation|GetActorLocation))
  (if (<= (Math|Vector|VectorLength (- (Variables|Default|GetLocationThisFrame) (Variables|Default|GetLocationLastFrame))) (Variables|Default|GetMinDistancePerFrame))
    (Audio|SpawnSoundatLocation (Variables|Default|GetImpactSound) (Variables|Default|GetLocationThisFrame) "0, 0, 0" 1.0 1.0 0.0 0 0)
    (Niagara|SpawnSystematLocation (Variables|Default|GetImpactEffect) (Variables|Default|GetLocationThisFrame))
    (Actor|DestroyActor)))