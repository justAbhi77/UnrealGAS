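; Arcane Shards gameplay ability: shows a magic circle, then on input press casts a series of damaging shards around the targeted ground point.
; A spawned BP_PointCollection supplies shuffled, randomly rotated points, their count scaling with ability level up to a cap.
; A montage event starts a looping timer that applies radial damage with knockback and fires a GameplayCue per point.
; Cost commits as shards start; cooldown commits after the last.
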(event Custom|eSpawnShard
  (bind _returnvalue (Ability|GetAvatarActorfromActorInfo))
  (if (< (Variables|Default|GetCurrentNumPoint) (Variables|Default|GetNumPoints))
    (Utilities|FlowControl|Sequence
      (:then_0
        (bind _output_get (Variables|Default|SetShardSpawnLocation (Transformation|GetWorldLocation (Utilities|Array|Get(acopy) (Variables|Default|GetGroundPoints) (Variables|Default|GetCurrentNumPoint)))))
        (Rendering|Debug|DrawDebugSphere _output_get 5e+01 12 "(R=1.000000,G=1.000000,B=1.000000,A=1.000000)" 3.0)
        (Utilities|FlowControl|Sequence
          (:then_0
            (bind _outoverlappingactors (Class|AuraAbilitySystemLibrary|GetLivePlayersWithinRadius _returnvalue (Utilities|Array|MakeArray _returnvalue) (Variables|Default|GetRadialDamageOuterRadius) (Variables|Default|GetShardSpawnLocation)))
            (bind _output_get_2 (Variables|Default|SetOverlappingActors _outoverlappingactors))
            (for _array_element _output_get_2
              (Class|AuraAbilitySystemLibrary|ApplyDamageEffect (Class|AuraDamageGameplayAbility|MakeDamageEffectParamsfromClassDefaults _array_element (Variables|Default|GetShardSpawnLocation) true (- (Transformation|GetActorLocation _array_element) (Variables|Default|GetShardSpawnLocation)) true (- (Transformation|GetActorLocation _array_element) (Variables|Default|GetShardSpawnLocation)) true 35.0))))
          (:then_1
            (Class|GameplayAbility|ExecuteGameplayCuewithParams "(TagName=\"GameplayCue.ArcaneShards\")" (Ability|GameplayCue|MakeGameplayCueParameters :Location (Variables|Default|GetShardSpawnLocation))))))
      (:then_1
        (Math|Integer|IncrementInt (Variables|Default|GetCurrentNumPoint))))
    (else
      (Utilities|FlowControl|Sequence
        (:then_0
          (Utilities|Time|ClearandInvalidateTimerbyHandle (Variables|Default|GetTimerHandle)))
        (:then_1
          (Ability|CommitAbilityCooldown false)
          (Actor|DestroyActor (Variables|Default|GetBpPointCollection))
          (Ability|EndAbility))))))

(event Ability|EventActivateAbility
  (bind _returnvalue (Class|GameplayAbility|CheckAbilityCost))
  (if _returnvalue
    (Utilities|FlowControl|Sequence
      (:then_0
        (Class|PlayerInterface|ShowMagicCircle(Message) (Ability|GetAvatarActorfromActorInfo) 0)
        (Variables|Default|SetCurrentNumPoint 0))
      (:then_1
        (Ability|Tasks|WaitInputPress false
          (:OnPress
            (Class|PlayerInterface|HideMagicCircle(Message) (Ability|GetAvatarActorfromActorInfo))
            (Utilities|FlowControl|Sequence
              (:then_0
                (bind _datahandle (|TargetDataUnderMouse)
                  (:ValidData
                    (Variables|Default|SetMouseHitLocation (.ImpactPoint (Collision|BreakHitResult (Ability|TargetData|GetHitResultfromTargetData _datahandle))))
                    (bind _returnvalue_2 (Game|SpawnActorfromClass "/Game/Blueprints/AbilitySystem/Aura/Abilities/Arcane/ArcaneShards/BP_PointCollection.BP_PointCollection_C" (Math|Transform|MakeTransform (Variables|Default|GetMouseHitLocation) "0, 0, 0" "1.000000,1.000000,1.000000") "AlwaysSpawn" "MultiplyWithRoot" 0 0))
                    (bind _output_get (Variables|Default|SetBpPointCollection _returnvalue_2))
                    (bind _output_get_2 (Variables|Default|SetNumPoints (Math|Integer|Min(Integer) (Variables|Default|GetMaxNumShards) (Ability|GetAbilityLevel))))
                    (bind _output_get_3 (Variables|Default|SetGroundPoints (Class|PointCollection|GetGroundPoints _output_get _output_get_2 (Math|Random|RandomFloatinRange 0.0 3.6e+02))))
                    (Utilities|Array|Shuffle _output_get_3)
                    (Utilities|FlowControl|Sequence
                      (:then_0
                        (Class|CombatInterface|UpdateFacingTarget(Message) (Ability|GetAvatarActorfromActorInfo) (Variables|Default|GetMouseHitLocation)))
                      (:then_1
                        (|PlayMontageandWaitProxy "None" "/Game/Assets/Characters/Aura/Animations/Abilities/AM_Cast_ArcaneShards.AM_Cast_ArcaneShards" 1.0 "None" false 1.0 0.0 false
                          (:then
                            (Ability|Tasks|WaitGameplayEvent "(TagName=\"Event.Montage.ArcaneShards\")" 0 true
                              (:EventReceived
                                (bind _returnvalue_3 (Utilities|Time|SetTimerbyEvent (delegate Custom|eSpawnShard) (Variables|Default|GetShardSpawnDeltaTime) true))
                                (Variables|Default|SetTimerHandle _returnvalue_3)
                                (CallFunction|ESpawnShard)
                                (Ability|CommitAbilityCost false)))))))))))))))))