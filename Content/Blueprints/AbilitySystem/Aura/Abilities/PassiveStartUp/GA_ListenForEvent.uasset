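; GA_ListenForEvent is a passive ability that listens for attribute gameplay events and applies them to its owner as a gameplay effect.
; On activation it waits for events under the Attributes tag, accepting child tags.
; Each event builds a spec from EventbasedEffectClass, sets the event tag and magnitude as a SetByCaller value, and applies it to self.
; Debug prints log listening and received tags.
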(event Ability|EventActivateAbility
  (bind _returnvalue (Ability|GetAbilitySystemComponentfromActorInfo))
  (Development|PrintString "Listening for events")
  (bind _payload (Ability|Tasks|WaitGameplayEvent "(TagName=\"Attributes\")" 0 false false)
    (:EventReceived
      (Development|PrintString (GameplayTags|GetDebugStringfromGameplayTag (.EventTag (Utilities|Struct|BreakGameplayEventData _payload))))
      (bind _returnvalue_2 (Ability|GameplayEffect|AssignTagSetbyCallerMagnitude (GameplayEffects|MakeOutgoingSpec _returnvalue (Variables|Default|GetEventbasedEffectClass) 1.0 (GameplayEffects|MakeEffectContext _returnvalue)) (.EventTag (Utilities|Struct|BreakGameplayEventData _payload)) (.EventMagnitude (Utilities|Struct|BreakGameplayEventData _payload))))
      (GameplayEffects|ApplyGameplayEffectSpecToSelf (Ability|GetAbilitySystemComponentfromActorInfo) _returnvalue_2))))