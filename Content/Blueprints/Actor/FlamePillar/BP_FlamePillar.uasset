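; BP_FlamePillar is a flame pillar actor whose fire light flickers continuously during play.
; A timeline curve scaled by a base intensity drives the Firelight intensity each update.
; Each cycle sets the timeline play rate from the inverse playback time plus a random variance, then restarts on finish, so the flicker speed varies between loops.
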(event Custom|eChangePlayBackSpeed
  (Components|Timeline|SetPlayRate (Variables|Default|GetTimeline-FlameIntensity) (+ (/ 1.0 (Variables|Public|GetPlayBackTime)) (Math|Random|RandomFloatinRange (Variables|Public|GetRandomVarianceMin) (Variables|Public|GetRandomVarianceMax))))
  (bind _flameintensity (Timeline|Timeline-FlameIntensity PlayFromStart)
    (:Update
      (Rendering|Components|Light|SetIntensity (Variables|Default|GetFirelight) (* _flameintensity (Variables|Public|GetBaseIntensity))))
    (:Finished
      (CallFunction|EChangePlayBackSpeed))))

(event EventBeginPlay
  (Components|Timeline|SetPlayRate (Variables|Default|GetTimeline-FlameIntensity) (+ (/ 1.0 (Variables|Public|GetPlayBackTime)) (Math|Random|RandomFloatinRange (Variables|Public|GetRandomVarianceMin) (Variables|Public|GetRandomVarianceMax))))
  (bind _flameintensity (Timeline|Timeline-FlameIntensity PlayFromStart)
    (:Update
      (Rendering|Components|Light|SetIntensity (Variables|Default|GetFirelight) (* _flameintensity (Variables|Public|GetBaseIntensity))))
    (:Finished
      (CallFunction|EChangePlayBackSpeed))))

(fn ConstructionScript)