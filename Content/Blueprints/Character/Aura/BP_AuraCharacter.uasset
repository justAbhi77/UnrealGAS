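; Player character Blueprint for Aura, adding camera-occlusion fading and motion-warped facing.
; A Box volume is resized and offset every tick to span half the camera boom's arm length along X, covering the camera-to-character line.
; Actors implementing BI_FadeInterface get fade-out and fade-in messages on entering and leaving the box.
; UpdateFacingTarget sets the FacingTarget warp target location for Motion Warping.
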(event OnComponentBeginOverlap(Box)
  (params (OverlappedComponent :type Primitive%20Component%20Object%20Reference) (OtherActor :type Actor%20Object%20Reference) (OtherComp :type Primitive%20Component%20Object%20Reference) (OtherBodyIndex :type Integer) (bFromSweep :type Boolean) (SweepResult :type Hit%20Result%20Structure%20%28by%20ref%29))
  (if (Utilities|DoesObjectImplementInterface OtherActor "/Game/Blueprints/Actor/FadeActor/BI_FadeInterface.BI_FadeInterface_C")
    (Class|BIFadeInterface|FadeOut(Message) OtherActor)))

(event OnComponentEndOverlap(Box)
  (params (OverlappedComponent :type Primitive%20Component%20Object%20Reference) (OtherActor :type Actor%20Object%20Reference) (OtherComp :type Primitive%20Component%20Object%20Reference) (OtherBodyIndex :type Integer))
  (if (Utilities|DoesObjectImplementInterface OtherActor "/Game/Blueprints/Actor/FadeActor/BI_FadeInterface.BI_FadeInterface_C")
    (Class|BIFadeInterface|Fadein(Message) OtherActor)))

(event EventUpdateFacingTarget
  (params (Target :type Vector%20%28by%20ref%29 :default "0, 0, 0"))
  (Class|MotionWarpingComponent|AddorUpdateWarpTargetfromLocation (Variables|Default|GetMotionWarping) "FacingTarget" Target))

(event EventTick
  (params (DeltaSeconds :type Float%20%28single-precision%29))
  (|CallParentFunction DeltaSeconds)
  (CallFunction|FSetSpringArmLength (Variables|/Script/Engine.SpringArmComponent|GetTargetArmLength (Variables|Default|GetCameraBoom))))

(event EventBeginPlay
  (|CallParentFunction)
  (CallFunction|FSetSpringArmLength (Variables|/Script/Engine.SpringArmComponent|GetTargetArmLength (Variables|Default|GetCameraBoom))))

(fn ConstructionScript)

(fn FSetSpringArmLength
  (params (TargetArmLength :type Float%20%28single-precision%29))
  (bind _box (Variables|Default|GetBox))
  (bind _relativelocation (Variables|/Script/Engine.SceneComponent|GetRelativeLocation _box))
  (bind _box_2 (Variables|Default|GetBox)
    (:then
      (LocalVariables|SetHalfTargetArmLength (/ (Variables|/Script/Engine.SpringArmComponent|GetTargetArmLength (Variables|Default|GetCameraBoom)) 2.0))
      (Components|Box|SetBoxExtent _box_2 (Math|Vector|MakeVector (LocalVariables|GetHalfTargetArmLength) (.y (Variables|/Script/Engine.BoxComponent|GetBoxExtent _box_2)) (.z (Variables|/Script/Engine.BoxComponent|GetBoxExtent _box_2))) true)
      (Transformation|SetRelativeLocation _box (Math|Vector|MakeVector (LocalVariables|GetHalfTargetArmLength) (.y _relativelocation) (.z _relativelocation)) false false))
    (:else)))