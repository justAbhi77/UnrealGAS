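; Base enemy character Blueprint that handles dissolve effects, attack-facing motion warping and loot drops.
; Two timelines drive the Dissolve parameter on body and weapon dynamic materials, and UpdateFacingTarget sets the FacingTarget warp location.
; SpawnLoot rolls items from loot tiers, then a looping timer spawns them one by one in an evenly spaced, floor-snapped ring at random distances.
; Flagged AuraEffectActor drops inherit the enemy's level.
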(event Custom|eSpawnLoot
  (bind _lootitems (Variables|Default|GetLootItems))
  (bind _spawnlootnum (Variables|Default|GetSpawnLootNum))
  (bind _output (Utilities|Array|Get(acopy) _lootitems _spawnlootnum))
  (bind (_lootclass _blootleveloverride) (Utilities|Struct|BreakLootItem _output))
  (if (< (Variables|Default|GetSpawnLootNum) (Utilities|Array|Length (Variables|Default|GetLootItems)))
    (Variables|Default|SetbWillOverrideLootLevel _blootleveloverride)
    (bind _returnvalue (Game|SpawnActorfromClass _lootclass (CallFunction|FGetSpawnTransform (Variables|Default|GetSpawnLootNum)) "AlwaysSpawn" "MultiplyWithRoot" 0 0))
    (Utilities|FlowControl|Sequence
      (:then_0
        (if (Variables|Default|GetbWillOverrideLootLevel)
          (bind _asaura_effect_actor (Utilities|Casting|CastToAuraEffectActor _returnvalue))
          (Variables|/Script/Aura.AuraEffectActor|SetActorLevel _asaura_effect_actor (Math|Conversions|ToFloat(Integer) (Variables|Default|GetLevel)))))
      (:then_1
        (Math|Integer|IncrementInt (Variables|Default|GetSpawnLootNum))))
    (else
      (Utilities|Time|ClearandInvalidateTimerbyHandle (Variables|Default|GetLootTimer)))))

(event EventStartDissolveTimeline
  (params (DynamicMaterialInstance :type Material%20Instance%20Dynamic%20Object%20Reference))
  (bind _dissolve (Timeline|Dissolve_Timeline Play)
    (:Update
      (Rendering|Material|SetScalarParameterValue DynamicMaterialInstance "Dissolve" _dissolve :!class /Script/Engine.MaterialInstanceDynamic))))

(event EventStartWeaponDissolveTimeline
  (params (DynamicMaterialInstance :type Material%20Instance%20Dynamic%20Object%20Reference))
  (bind _weapondissolve (Timeline|WeaponDissolve_Timeline Play)
    (:Update
      (Rendering|Material|SetScalarParameterValue DynamicMaterialInstance "Dissolve" _weapondissolve :!class /Script/Engine.MaterialInstanceDynamic))))

(event EventUpdateFacingTarget
  (params (Target :type Vector%20%28by%20ref%29 :default "0, 0, 0"))
  (Class|MotionWarpingComponent|AddorUpdateWarpTargetfromLocation (Variables|Default|GetMotionWarping) "FacingTarget" Target))

(event EventBeginPlay
  (|CallParentFunction))

(event EventSpawnLoot
  (bind _returnvalue (Class|AuraAbilitySystemLibrary|GetLootTiers))
  (Utilities|IsValid _returnvalue
    (:Is%20Valid
      (bind _returnvalue_2 (Class|LootTiers|GetLootItems _returnvalue))
      (bind _output_get (Variables|Default|SetLootItems _returnvalue_2))
      (Variables|Default|SetActorForward (Transformation|GetActorForwardVector))
      (Variables|Default|SetLootRotations (CallFunction|FGetLootRotations _output_get))
      (Variables|Default|SetSpawnLootNum 0)
      (Variables|Default|SetActorLocation (Transformation|GetActorLocation))
      (bind _returnvalue_3 (Utilities|Time|SetTimerbyEvent (delegate Custom|eSpawnLoot) 0.1 true))
      (Variables|Default|SetLootTimer _returnvalue_3)
      (CallFunction|ESpawnLoot))))

(fn ConstructionScript
  (|CallParentFunction))

(fn FGetLootRotations
  (params (TargetArray :type Array%20of%20Loot%20Item%20Structures))
  (return (Class|AuraAbilitySystemLibrary|EvenlySpacedRotators (Variables|Default|GetActorForward) (Math|Vector|VectorUp) 3.6e+02 (Utilities|Array|Length TargetArray))))

(fn FGetSpawnTransform
  (params (SpawnNum :type Integer))
  (bind _lootrotations (Variables|Default|GetLootRotations))
  (bind _output (Utilities|Array|Get(acopy) _lootrotations SpawnNum))
  (return (Math|Transform|MakeTransform (.OutClosestLocation (Class|AuraAbilitySystemLibrary|FindClosestLocationonFloor 0 (+ (Variables|Default|GetActorLocation) (* (Math|Random|RandomFloatinRange (Variables|Default|GetMinSpawnDistance) (Variables|Default|GetMaxSpawnDistance)) (Math|Vector|GetForwardVector _output))) 4e+02 5e+01)) _output)))