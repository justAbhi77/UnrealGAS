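; BP_Aura_MainMenu is the actor that sets up the main menu and animates a floating fireball in its scene.
; On BeginPlay it plays the menu music, adds WBP_MainMenu to the viewport, and switches to UI-only input with a visible cursor.
; Each Tick advances a timer that wraps after 2π, bobbing the fireball vertically on a sine wave around its starting location.
; A magic circle decal rotation exists but is never executed.
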(event EventBeginPlay
  (bind _returnvalue (Game|GetPlayerController 0))
  (Variables|Private|SetFireballInitialLocation (Transformation|GetWorldLocation (Variables|Default|GetFireball)))
  (Audio|PlaySound2D "/Game/Assets/Sounds/Music/Music_MainMenu.Music_MainMenu" 1.0 1.0 0.0 0 0)
  (bind _returnvalue_2 (UserInterface|CreateWidget "/Game/Blueprints/UI/MainMenu/WBP_MainMenu.WBP_MainMenu_C" (Game|GetPlayerController 0)))
  (UserInterface|Viewport|AddtoViewport _returnvalue_2 0)
  (Input|SetInputModeUIOnly _returnvalue _returnvalue_2 "LockOnCapture" false)
  (Variables|/Script/Engine.PlayerController|SetbShowMouseCursor _returnvalue true))

(event EventTick
  (params (DeltaSeconds :type Float%20%28single-precision%29))
  (CallFunction|UpdateTime DeltaSeconds)
  (Transformation|SetWorldLocation (Variables|Default|GetFireball) (+ (Variables|Private|GetFireballInitialLocation) (Math|Vector|MakeVector 0.0 0.0 (CallFunction|SinTime))) false false))

(fn ConstructionScript)

(fn UpdateTime
  (params (A :type Float%20%28double-precision%29))
  (bind _output_get (Variables|Private|SetTime (+ A (Variables|Private|GetTime))))
  (if (> _output_get 6.28318)
    (Variables|Private|SetTime 0.0)))

(fn SinTime
  (return (* (Math|Trig|Sin(Radians) (Variables|Private|GetTime)) (Variables|Public|GetAmplitude))))